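; Base character Blueprint that handles movement scaling, health, passive regeneration and death.
; BeginPlay applies speed and jump scales to the CharacterMovement component and fills health to maximum.
; Tick regenerates health up to the maximum until death, and TakeDamage subtracts from it through UpdateHealth.
; Health at or below zero calls Die, which only sets IsDead and prints a red debug message.
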(event `self.ReceiveBeginPlay`
  (`self.Update Movement Speed` (`self.movementSpeedScale`) (`self.jumpForceScale`))
  (`self.UpdateHealth` (`self.maxHealth`)))

(event `self.ReceiveTick`
  (params (DeltaSeconds :type "Float (single-precision)"))
  (`self.Recover` (* DeltaSeconds (`self.passiveRecoveryAmount`))))

(fn `Die`
  (`KismetSystemLibrary.PrintString` "YOU ARE DED" true true (struct :`R` 1.0 :`A` 1.0) 200.0)
  (set `self.isDead` true))

(fn `Recover`
  (params (RecoverAmount :type "Float (double-precision)"))
  (if (not (`self.isDead`))
    (`self.UpdateHealth` (`KismetMathLibrary.FClamp` (+ RecoverAmount (`self.currentHealth`)) -500.0 (`self.maxHealth`)))))

(fn `TakeDamage`
  (params (DamageTaken :type "Float (double-precision)"))
  (`self.UpdateHealth` (- (`self.currentHealth`) DamageTaken)))

(fn `Update Movement Speed`
  (params (`New Movement Speed Scale` :type "Float (double-precision)") (`New Jump Force Scale` :type "Float (double-precision)"))
  (bind _charactermovement (`self.CharacterMovement`))
  ; Max movement speed update
  (set `CharacterMovementComponent.MaxWalkSpeed` (* 600.0 `New Movement Speed Scale`) (`self.CharacterMovement`))
  ; Max movement acceleration update
  (set `CharacterMovementComponent.MaxAcceleration` (* 2048.0 `New Movement Speed Scale`) (`self.CharacterMovement`))
  ; Jump force update
  (set `CharacterMovementComponent.JumpZVelocity` (* (`CharacterMovementComponent.JumpZVelocity` _charactermovement) `New Jump Force Scale`) _charactermovement))

(fn `UpdateHealth`
  (params (NewValue :type "Float (double-precision)"))
  (if (> NewValue 0.0)
    (set `self.currentHealth` NewValue)
    (else
      (`self.Die`)
      (set `self.currentHealth` NewValue))))

(fn `UserConstructionScript`)