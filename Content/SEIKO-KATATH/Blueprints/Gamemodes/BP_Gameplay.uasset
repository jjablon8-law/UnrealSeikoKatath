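; BP_Gameplay is a gameplay game mode Blueprint that handles the opening instructions screen, the game GUI and level changes.
; On BeginPlay it pauses the game, adds the instructions widget to the player's screen and shows the mouse cursor.
; A ShowGameGUI event creates the game GUI widget and adds it to the viewport, and a ChangeLevel function opens a level by name.
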(event `self.ReceiveBeginPlay`
  (`GameplayStatics.SetGamePaused` true)
  (bind _returnvalue (`|CreateWidget` "/Game/SEIKO-KATATH/Blueprints/Widgets/BP_Instructions_Widget.BP_Instructions_Widget_C" (`GameplayStatics.GetPlayerController` 0)))
  (`UserWidget.AddToPlayerScreen` _returnvalue 0)
  (set `PlayerController.bShowMouseCursor` true (`GameplayStatics.GetPlayerController` 0)))

(event `Show GameGUI`
  (bind _returnvalue (`|CreateWidget` "/Game/SEIKO-KATATH/Blueprints/Widgets/BP_GameGUI_Widget.BP_GameGUI_Widget_C"))
  (`UserWidget.AddToViewport` _returnvalue 0))

(fn `ChangeLevel`
  (params (LevelName :type Name))
  (`GameplayStatics.OpenLevel` LevelName))

(fn `UserConstructionScript`)